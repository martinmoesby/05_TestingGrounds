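; AI controller Blueprint for a guard NPC that runs the GuardBehaviour tree with the PatrolData blackboard from BeginPlay.
; Perception updates write any actor lacking the "Enemy" tag to the blackboard's EnemyKey when sensed, and clear the key when sensing fails.
; A debug helper, not called in these graphs, prints the controller name, sense class and perceived object.
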(event OnTargetPerceptionUpdated(AIPerception)
  (params (Actor :type Actor%20Object%20Reference) (Stimulus :type AI%20Stimulus%20Structure))
  (bind _enemykey (Variables|Default|GetEnemyKey))
  (bind _blackboardcomp (Variables|Default|GetBlackboardComp))
  ;[1 1 1] Set or clear enemy actor
  (if (not (Actor|ActorHasTag Actor "Enemy"))
    (if (.bSuccessfullySensed (Utilities|Struct|BreakAIStimulus Stimulus))
      (AI|Components|Blackboard|SetValueasObject _blackboardcomp _enemykey Actor)
      (else
        (AI|Components|Blackboard|ClearValue _blackboardcomp _enemykey)))))

(event EventBeginPlay
  (bind _blackboardcomponent (Class|AIController|UseBlackboard "/Game/Dynamic/Character/AI/PatrolData.PatrolData"))
  (Variables|Default|SetBlackboardComp _blackboardcomponent)
  (AI|RunBehaviorTree "/Game/Dynamic/Character/AI/BehaviourTrees/GuardBehaviour.GuardBehaviour"))

(fn ConstructionScript)

(fn PrintPerceptionInfoDEBUG
  (params (Object :type Object%20Object%20Reference) (Stimulus :type AI%20Stimulus%20Structure%20%28by%20ref%29))
  (bind _returnvalue (Class|AIPerceptionSystem|GetSenseClassforStimulus Stimulus))
  (Development|PrintString (Utilities|String|Append (Utilities|GetObjectName self) " " (Utilities|GetClassDisplayName _returnvalue) " " (Utilities|GetDisplayName Object))))